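; Base item actor that the player can pick up, inspect up close and drop, showing a named prompt on look-at.
; Interacting attaches it to the player's grip, or starts inspection if something is already held.
; Inspection swaps the HUD for a description widget and takes over input for mouse-drag rotation and wheel zoom along camera forward.
; Stopping restores input, HUD and relative transform; dropping detaches it and re-enables physics.
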(event EventLookat
  (params (PlayerCharacter :type First%20Person%20Character%20Object%20Reference))
  (Default|UpdateMessage (Variables|/Game/FirstPersonBP/Blueprints/FirstPersonCharacter.FirstPersonCharacter_C|GetHUD PlayerCharacter) (Utilities|Text|FormatText "Press E to Pick Up {name}" (Variables|Default|GetItemName))))

(event EventInteractwith
  (params (PlayerCharacter :type First%20Person%20Character%20Object%20Reference))
  (bind _output_get (Variables|Default|SetPlayer PlayerCharacter))
  (Variables|/Game/FirstPersonBP/Blueprints/FirstPersonCharacter.FirstPersonCharacter_C|GetCurrentlyHeldItem _output_get
    (:then
      (CallFunction|StartInspect))
    (:else
      (CallFunction|PickUpItem))))

(event Input|ActionEvents|InputActionInteract
  (params (Key :type Key%20Structure))
  (:Pressed
    (CallFunction|StopInspect)))

(event Input|MouseEvents|MouseX
  (params (AxisValue :type Float%20%28single-precision%29))
  ;[1 1 1] Rotating X-Axis
  (if (Variables|Default|GetisRotating)
    (Transformation|SetActorRotation (Math|Rotator|CombineRotators (Transformation|GetActorRotation) (Math|Rotator|MakeRotator 0.0 0.0 (* AxisValue (Variables|Default|GetMouseRotationValue)))))))

(event Input|MouseEvents|MouseY
  (params (AxisValue :type Float%20%28single-precision%29))
  ;[1 1 1] Rotating Y-Axis
  (if (Variables|Default|GetisRotating)
    (Transformation|SetActorRotation (Math|Rotator|CombineRotators (Transformation|GetActorRotation) (Math|Rotator|MakeRotator 0.0 (* AxisValue (Variables|Default|GetMouseRotationValue)) 0.0)))))

(event Input|MouseEvents|LeftMouseButton
  (params (Key :type Key%20Structure))
  (:Pressed
    (Variables|Default|SetisRotating true))
  (:Released
    (Variables|Default|SetisRotating false)))

(event Input|MouseEvents|MouseWheelUp
  (params (Key :type Key%20Structure))
  (bind _returnvalue (Game|GetPlayerCameraManager 0))
  ;[1 1 1] Zoom in
  (:Pressed
    (bind _output_get (Variables|Default|SetZoomLevel (Math|Integer|Clamp(Integer) (+ (Variables|Default|GetZoomLevel) (Variables|Default|GetZoomAdd)) (Variables|Default|GetZoomMinValue) (Variables|Default|GetZoomMaxValue))))
    (if (< _output_get (Variables|Default|GetZoomMaxValue))
      (Transformation|SetActorLocation (+ (Camera|GetCameraLocation _returnvalue) (* (Math|Vector|GetForwardVector (Camera|GetCameraRotation _returnvalue)) (* (Variables|Default|GetZoomLevel) (Variables|Default|GetZoomSpeed)))) false false))))

(event Input|MouseEvents|MouseWheelDown
  (params (Key :type Key%20Structure))
  (bind _returnvalue (Game|GetPlayerCameraManager 0))
  ;[1 1 1] Zoom out
  (:Pressed
    (bind _output_get (Variables|Default|SetZoomLevel (Math|Integer|Clamp(Integer) (- (Variables|Default|GetZoomLevel) (Variables|Default|GetZoomAdd)) (Variables|Default|GetZoomMinValue) (Variables|Default|GetZoomMaxValue))))
    (if (> _output_get (Variables|Default|GetZoomMinValue))
      (Transformation|SetActorLocation (+ (Camera|GetCameraLocation _returnvalue) (* (Math|Vector|GetForwardVector (Camera|GetCameraRotation _returnvalue)) (* (Variables|Default|GetZoomLevel) (Variables|Default|GetZoomSpeed)))) false false))))

(fn ConstructionScript)

(fn PickUpItem
  (Transformation|AttachComponentToComponent (Variables|/Game/FirstPersonBP/Blueprints/FirstPersonCharacter.FirstPersonCharacter_C|GetItemGrip (Variables|Default|GetPlayer)) "None" "SnapToTarget" "SnapToTarget" "KeepRelative" true)
  (Physics|SetSimulatePhysics (Variables|Default|GetStaticMesh) false)
  (Collision|SetCollisionEnabled (Variables|Default|GetStaticMesh) "NoCollision")
  (Variables|/Game/FirstPersonBP/Blueprints/FirstPersonCharacter.FirstPersonCharacter_C|SetCurrentlyHeldItem (Variables|Default|GetPlayer) self))

(fn StartInspect
  (bind _returnvalue (Game|GetPlayerController 0))
  (bind _returnvalue_2 (Game|GetPlayerCameraManager 0))
  (Widget|SetVisibility (Variables|/Game/FirstPersonBP/Blueprints/FirstPersonCharacter.FirstPersonCharacter_C|GetHUD (Variables|Default|GetPlayer)) "Hidden")
  (bind _returnvalue_3 (UserInterface|CreateWidget "/Game/UI/InspectionScreen.InspectionScreen_C" 0 (Variables|Default|GetItemDescription)))
  (bind _output_get (Variables|Default|SetInspectionUI _returnvalue_3))
  (UserInterface|Viewport|AddtoViewport _output_get 0)
  (Input|DisableInput (Variables|Default|GetPlayer) _returnvalue)
  (Input|EnableInput _returnvalue)
  (Transformation|SetActorLocation (+ (Camera|GetCameraLocation _returnvalue_2) (* (Math|Vector|GetForwardVector (Camera|GetCameraRotation _returnvalue_2)) (Variables|Default|GetInspectionDistance))) false false))

(fn DropItem
  (bind _returnvalue (Game|GetPlayerCameraManager 0))
  (bind _staticmesh (Variables|Default|GetStaticMesh))
  (Transformation|DetachFromActor "KeepWorld" "KeepWorld" "KeepWorld")
  (Transformation|SetActorLocation (+ (Camera|GetCameraLocation _returnvalue) (* (Math|Vector|GetForwardVector (Camera|GetCameraRotation _returnvalue)) (Variables|Default|GetInspectionDistance))) false false)
  (Physics|SetSimulatePhysics _staticmesh true)
  (Collision|SetCollisionEnabled _staticmesh "QueryAndPhysics"))

(fn StopInspect
  (bind _returnvalue (Game|GetPlayerController 0))
  (Input|DisableInput _returnvalue)
  (Input|EnableInput (Variables|Default|GetPlayer) _returnvalue)
  (Transformation|SetActorRelativeLocation "0, 0, 0")
  (Transformation|SetActorRelativeRotation "0, 0, 0")
  (Widget|RemovefromParent (Variables|Default|GetInspectionUI))
  (Widget|SetVisibility (Variables|/Game/FirstPersonBP/Blueprints/FirstPersonCharacter.FirstPersonCharacter_C|GetHUD (Variables|Default|GetPlayer)) "Visible"))