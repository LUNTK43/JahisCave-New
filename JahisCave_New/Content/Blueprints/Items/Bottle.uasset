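; Bottle item that the player can pick up and inspect, with no active event graph logic.
; PickUpItem snaps it to the player's ItemGrip, turns off mesh physics and collision, and sets the player's CurrentlyHeldItem to None rather than to the bottle.
; StopInspect hands input back to the player, zeroes the bottle's relative transform, removes the inspection UI and shows the HUD again.
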(event EventBeginPlay)

(event Collision|EventActorBeginOverlap
  (params (OtherActor :type Actor%20Object%20Reference)))

(event EventTick
  (params (DeltaSeconds :type Float%20%28single-precision%29)))

(fn ConstructionScript)

(fn StopInspect
  (bind _returnvalue (Game|GetPlayerController 0))
  (Input|DisableInput _returnvalue)
  (Input|EnableInput (Variables|Default|GetPlayer) _returnvalue)
  (Transformation|SetActorRelativeLocation "0, 0, 0")
  (Transformation|SetActorRelativeRotation "0, 0, 0")
  (Widget|RemovefromParent (Variables|Default|GetInspectionUI))
  (Widget|SetVisibility (Variables|/Game/FirstPersonBP/Blueprints/FirstPersonCharacter.FirstPersonCharacter_C|GetHUD (Variables|Default|GetPlayer)) "Visible"))

(fn PickUpItem
  (Transformation|AttachComponentToComponent (Variables|/Game/FirstPersonBP/Blueprints/FirstPersonCharacter.FirstPersonCharacter_C|GetItemGrip (Variables|Default|GetPlayer)) "None" "SnapToTarget" "SnapToTarget" "KeepRelative" true)
  (Physics|SetSimulatePhysics (Variables|Mesh|GetStaticMesh) false)
  (Collision|SetCollisionEnabled (Variables|Mesh|GetStaticMesh) "NoCollision")
  (Variables|/Game/FirstPersonBP/Blueprints/FirstPersonCharacter.FirstPersonCharacter_C|SetCurrentlyHeldItem (Variables|Default|GetPlayer) 0 self))