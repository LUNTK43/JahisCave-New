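; Level transition actor: an interactable door that loads another level when the player walks into it.
; Look-at shows an "open" prompt on the player's HUD, and interacting plays a timeline that moves the door mesh along Z.
; First-person character overlap opens the referenced level, passing a destination tag as the options string, independent of door state.
; Key-check logic that would consume a held key is present but disconnected.
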(event Custom|OpenDoor
  (bind _doorheight (Timeline|DoorPosition Play)
    (:Update
      (Transformation|SetRelativeLocation (Variables|Default|GetDoor) (Math|Vector|MakeVector 0.0 0.0 _doorheight) false false))))

(event EventBeginPlay)

(event Collision|EventActorBeginOverlap
  (params (OtherActor :type Actor%20Object%20Reference))
  (Utilities|Casting|CastToFirstPersonCharacter OtherActor)
  (Game|OpenLevel(byObjectReference) (Variables|Default|GetLevel) true (Variables|Default|GetDestinationTag)))

(event EventTick
  (params (DeltaSeconds :type Float%20%28single-precision%29)))

(event EventLookat
  (params (PlayerCharacter :type First%20Person%20Character%20Object%20Reference))
  (Default|UpdateMessage (Variables|/Game/FirstPersonBP/Blueprints/FirstPersonCharacter.FirstPersonCharacter_C|GetHUD PlayerCharacter) (Utilities|Text|FormatText "Press E to open {name}" (Variables|Default|GetDoor))))

(event EventInteractwith
  (params (PlayerCharacter :type First%20Person%20Character%20Object%20Reference))
  (CallFunction|OpenDoor))

(fn ConstructionScript)